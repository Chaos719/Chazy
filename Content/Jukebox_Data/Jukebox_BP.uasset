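; Jukebox Blueprint actor that plays a media playlist through a Media Player, controlled by the keyboard.
; On BeginPlay it enables input from the first player controller and opens the first entry of Jukebox_PL.
; N and B skip to the next and previous tracks, while P alternates pause and play through a FlipFlop, starting with pause.
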(event `self.ReceiveBeginPlay`
  (`self.EnableInput` (`GameplayStatics.GetPlayerController` 0))
  (`MediaPlayer.OpenPlaylistIndex` (`self.Media Player`) "/Game/Jukebox_Data/Jukebox_PL.Jukebox_PL" 0))

(event `Key|N`
  (params (Key :type "Key Structure"))
  (:`Pressed`
    (`MediaPlayer.Next` (`self.Media Player`))))

(event `Key|B`
  (params (Key :type "Key Structure"))
  (:`Pressed`
    (`MediaPlayer.Previous` (`self.Media Player`))))

(event `Key|P`
  (params (Key :type "Key Structure"))
  (bind _media_player (`self.Media Player`))
  (:`Pressed`
    (`/Engine/EditorBlueprintResources/StandardMacros.FlipFlop`
      (:`A`
        (`MediaPlayer.Pause` _media_player))
      (:`B`
        (`MediaPlayer.Play` _media_player)))))

(fn `UserConstructionScript`)