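; BP_QuizStation is a quiz station that locks the player in place and opens the quiz UI when they walk into its trigger.
; On TriggerBox overlap by a QuizCharacter, it disables movement, moves the character to the Arrow component and aligns control rotation with it.
; It then switches player 0 to UI-only input with a visible cursor and adds a new HUDQuiz widget.
; Nothing here restores movement or input.
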(event `self.TriggerBox.OnComponentBeginOverlap`
  (params (OverlappedComponent :type "PrimitiveComponent Object Reference") (OtherActor :type "Actor Object Reference") (OtherComp :type "PrimitiveComponent Object Reference") (OtherBodyIndex :type Integer) (bFromSweep :type Boolean) (SweepResult :type "HitResult Structure (by ref)"))
  (bind _returnvalue (`GameplayStatics.GetPlayerController` 0))
  (bind _arrow (`self.Arrow`))
  (bind _asquiz_character (cast `/Game/GameMode/QuizCharacter` OtherActor))
  (if (== OtherActor _asquiz_character)
    (`CharacterMovementComponent.DisableMovement` (`Character.CharacterMovement` _asquiz_character))
    (`SceneComponent.K2_SetWorldLocation` (`Actor.RootComponent` _asquiz_character) (`SceneComponent.K2_GetComponentLocation` _arrow) false false)
    (`Controller.SetControlRotation` _returnvalue (`SceneComponent.K2_GetComponentRotation` _arrow))
    (`WidgetBlueprintLibrary.SetInputMode_UIOnlyEx` _returnvalue null)
    (set `PlayerController.bShowMouseCursor` true _returnvalue)
    (bind _returnvalue_2 (`|CreateWidget` "/Game/Quiz/HUDQuiz.HUDQuiz_C" _returnvalue))
    (`UserWidget.AddToViewport` _returnvalue_2 0)))

(fn `UserConstructionScript`)