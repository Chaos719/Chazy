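; BP_WidgetTester is a trigger actor, apparently for testing widgets, that opens the EscapeMenuGrapple menu when the player character overlaps its Box.
; On overlap it creates the widget, adds it to the viewport, switches input to UI-only with the mouse cursor shown, and disables movement on the GrappleChar01 character.
; Nothing in this Blueprint closes the menu or restores input and movement.
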(event `self.Box.OnComponentBeginOverlap`
  (params (OverlappedComponent :type "PrimitiveComponent Object Reference") (OtherActor :type "Actor Object Reference") (OtherComp :type "PrimitiveComponent Object Reference") (OtherBodyIndex :type Integer) (bFromSweep :type Boolean) (SweepResult :type "HitResult Structure (by ref)"))
  (bind _returnvalue (`GameplayStatics.GetPlayerCharacter` 0))
  (bind _returnvalue_2 (`GameplayStatics.GetPlayerController` 0))
  (if (== _returnvalue OtherActor)
    (bind _returnvalue_3 (`|CreateWidget` "/Game/GrappleGame/EscapeMenuGrapple.EscapeMenuGrapple_C"))
    (`UserWidget.AddToViewport` _returnvalue_3 0)
    (`WidgetBlueprintLibrary.SetInputMode_UIOnlyEx` _returnvalue_2 _returnvalue_3)
    (set `PlayerController.bShowMouseCursor` true _returnvalue_2)
    (bind _asgrapple_char_01 (cast `/Game/FirstPersonBP/Blueprints/GrappleChar01` _returnvalue))
    (`CharacterMovementComponent.DisableMovement` (`Character.CharacterMovement` _asgrapple_char_01))))

(fn `UserConstructionScript`)